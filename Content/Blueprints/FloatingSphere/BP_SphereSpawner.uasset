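; A spawner actor that periodically creates BP_FloatingSphere actors at random points around itself.
; BeginPlay starts a looping timer at SpawnTime, and each firing spawns one sphere.
; Each location comes from the actor's position plus a random rotator's forward vector, scaled by a random distance up to SpawnRadius.
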(event Custom|SpawnSphereEvent
  (Game|SpawnActorfromClass "/Game/Blueprints/FloatingSphere/BP_FloatingSphere.BP_FloatingSphere_C" (Math|Transform|MakeTransform (CallFunction|GetRandomPointWithinASphereRadius) "0, 0, 0" "1.000000,1.000000,1.000000") "Undefined" "MultiplyWithRoot" 0 0))

(event EventBeginPlay
  (Utilities|Time|SetTimerbyEvent (delegate Custom|SpawnSphereEvent) (Variables|Default|GetSpawnTime) true))

(event EventTick
  (params (DeltaSeconds :type Float%20%28single-precision%29)))

(fn ConstructionScript)

(fn GetRandomPointWithinASphereRadius
  (return (+ (Transformation|GetActorLocation) (* (Math|Vector|GetForwardVector (Math|Random|RandomRotator false)) (Math|Random|RandomFloatinRange 0.0 (Variables|Default|GetSpawnRadius))))))