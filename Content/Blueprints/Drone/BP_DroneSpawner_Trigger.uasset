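; One-shot trigger actor that spawns drones when any actor begins overlapping it, then destroys itself.
; With IsBossSpawner set, it spawns a single BP_Boss_Drone at the first TargetPoints entry.
; Otherwise it spawns a BP_Drone at every target point, with DestroyActor wired inside the loop body rather than after completion.
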(event Collision|EventActorBeginOverlap
  (params (OtherActor :type Actor%20Object%20Reference))
  (if (Variables|Default|GetisBossSpawner)
    (Game|SpawnActorfromClass "/Game/Blueprints/Drone/BP_Boss_Drone.BP_Boss_Drone_C" (Transformation|GetActorTransform (Utilities|Array|Get(acopy) (Variables|Default|GetTargetPoints))) "Undefined" "MultiplyWithRoot" 0 0)
    (Actor|DestroyActor :!label _label)
    (else
      (for _array_element (Variables|Default|GetTargetPoints)
        (Game|SpawnActorfromClass "/Game/Blueprints/Drone/BP_Drone.BP_Drone_C" (Transformation|GetActorTransform _array_element) "Undefined" "MultiplyWithRoot" 0 0)
        (goto _label)))))

(fn ConstructionScript)