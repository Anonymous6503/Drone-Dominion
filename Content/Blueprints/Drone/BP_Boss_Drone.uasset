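; BP_Boss_Drone is a boss drone actor that tracks its own health and explodes when destroyed.
; It calls its parent's BeginPlay, then sets a high starting Health.
; Tick drives InterpRotation every frame to interpolate its rotation.
; GetHurt subtracts damage, and at zero health spawns a Niagara fire explosion with an impact sound before destroying the actor.
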(event EventBeginPlay
  (|CallParentFunction)
  (Variables|Default|SetHealth 5e+02))

(event Collision|EventActorBeginOverlap
  (params (OtherActor :type Actor%20Object%20Reference)))

(event EventTick
  (params (DeltaSeconds :type Float%20%28single-precision%29))
  (CallFunction|InterpRotation DeltaSeconds (Variables|Default|GetInterp%20Speed)))

(event EventGetHurt
  (params (Damage :type Float%20%28double-precision%29))
  (bind _output_get (Variables|Default|SetHealth (- (Variables|Default|GetHealth) Damage)))
  (if (<= _output_get 0.0)
    (Niagara|SpawnSystematLocation "/Game/Assets/Effects/Projectiles/FireExplosion/NS_FireExplosion.NS_FireExplosion" (Transformation|GetActorLocation))
    (Audio|PlaySoundatLocation "/Game/Assets/Sounds/Explode/sfx_FireBolt_Impact.sfx_FireBolt_Impact" (Transformation|GetActorLocation) "0, 0, 0" 1.0 1.0 0.0 0 0 0 0)
    (Actor|DestroyActor)))

(fn ConstructionScript
  (|CallParentFunction))